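; BP_Treasure is a treasure chest that opens its lid when the player pawn overlaps it.
; The overlap calls OpenLid, which plays a 2D creak sound and runs the LidOpening timeline.
; The timeline scales OpenAngle to roll LidHinge, then snaps it to the full angle when finished.
; Nothing closes the lid or guards against repeat overlaps, so the sound plays on each one.
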(event Custom|OpenLid
  (bind _openangle (Variables|Default|GetOpenAngle))
  (Audio|PlaySound2D "/Game/SFX/treasure_chest_creak.treasure_chest_creak" 1.0 1.0 0.0 0 0)
  (bind _lidrotation (Timeline|LidOpening Play)
    (:Update
      (Transformation|SetRelativeRotation (Variables|Default|GetLidHinge) (Math|Rotator|MakeRotator (* _lidrotation _openangle) 0.0 0.0) false false))
    (:Finished
      (Transformation|SetRelativeRotation (Variables|Default|GetLidHinge) (Math|Rotator|MakeRotator _openangle 0.0 0.0) false false))))

(event Collision|EventActorBeginOverlap
  (params (OtherActor :type Actor%20Object%20Reference))
  (if (== OtherActor (Game|Player|GetPlayerPawn 0))
    (CallFunction|OpenLid)))

(fn ConstructionScript)