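; BP_MapTile is a map tile actor that changes its appearance when the player reaches a tavern area.
; Seven TavernCollider components each check on begin overlap whether the other actor is the player 0 pawn.
; Any match swaps the StaticMesh's first material slot to M_Tavern through one shared node.
; The change has no end-overlap reversal, and the construction script is empty.
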(event OnComponentBeginOverlap(TavernCollider6)
  (params (OverlappedComponent :type Primitive%20Component%20Object%20Reference) (OtherActor :type Actor%20Object%20Reference) (OtherComp :type Primitive%20Component%20Object%20Reference) (OtherBodyIndex :type Integer) (bFromSweep :type Boolean) (SweepResult :type Hit%20Result%20Structure%20%28by%20ref%29))
  (if (== (Game|Player|GetPlayerPawn 0) OtherActor)
    (Rendering|Material|SetMaterial (Variables|Default|GetStaticMesh) 0 "/Game/Images/Maps/M_Tavern.M_Tavern")))

(event OnComponentBeginOverlap(TavernCollider1)
  (params (OverlappedComponent :type Primitive%20Component%20Object%20Reference) (OtherActor :type Actor%20Object%20Reference) (OtherComp :type Primitive%20Component%20Object%20Reference) (OtherBodyIndex :type Integer) (bFromSweep :type Boolean) (SweepResult :type Hit%20Result%20Structure%20%28by%20ref%29))
  (if (== (Game|Player|GetPlayerPawn 0) OtherActor)
    (Rendering|Material|SetMaterial (Variables|Default|GetStaticMesh) 0 "/Game/Images/Maps/M_Tavern.M_Tavern")))

(event OnComponentBeginOverlap(TavernCollider)
  (params (OverlappedComponent :type Primitive%20Component%20Object%20Reference) (OtherActor :type Actor%20Object%20Reference) (OtherComp :type Primitive%20Component%20Object%20Reference) (OtherBodyIndex :type Integer) (bFromSweep :type Boolean) (SweepResult :type Hit%20Result%20Structure%20%28by%20ref%29))
  (if (== (Game|Player|GetPlayerPawn 0) OtherActor)
    (Rendering|Material|SetMaterial (Variables|Default|GetStaticMesh) 0 "/Game/Images/Maps/M_Tavern.M_Tavern")))

(event OnComponentBeginOverlap(TavernCollider3)
  (params (OverlappedComponent :type Primitive%20Component%20Object%20Reference) (OtherActor :type Actor%20Object%20Reference) (OtherComp :type Primitive%20Component%20Object%20Reference) (OtherBodyIndex :type Integer) (bFromSweep :type Boolean) (SweepResult :type Hit%20Result%20Structure%20%28by%20ref%29))
  (if (== (Game|Player|GetPlayerPawn 0) OtherActor)
    (Rendering|Material|SetMaterial (Variables|Default|GetStaticMesh) 0 "/Game/Images/Maps/M_Tavern.M_Tavern")))

(event OnComponentBeginOverlap(TavernCollider4)
  (params (OverlappedComponent :type Primitive%20Component%20Object%20Reference) (OtherActor :type Actor%20Object%20Reference) (OtherComp :type Primitive%20Component%20Object%20Reference) (OtherBodyIndex :type Integer) (bFromSweep :type Boolean) (SweepResult :type Hit%20Result%20Structure%20%28by%20ref%29))
  (if (== (Game|Player|GetPlayerPawn 0) OtherActor)
    (Rendering|Material|SetMaterial (Variables|Default|GetStaticMesh) 0 "/Game/Images/Maps/M_Tavern.M_Tavern")))

(event OnComponentBeginOverlap(TavernCollider5)
  (params (OverlappedComponent :type Primitive%20Component%20Object%20Reference) (OtherActor :type Actor%20Object%20Reference) (OtherComp :type Primitive%20Component%20Object%20Reference) (OtherBodyIndex :type Integer) (bFromSweep :type Boolean) (SweepResult :type Hit%20Result%20Structure%20%28by%20ref%29))
  (if (== (Game|Player|GetPlayerPawn 0) OtherActor)
    (Rendering|Material|SetMaterial (Variables|Default|GetStaticMesh) 0 "/Game/Images/Maps/M_Tavern.M_Tavern")))

(event OnComponentBeginOverlap(TavernCollider2)
  (params (OverlappedComponent :type Primitive%20Component%20Object%20Reference) (OtherActor :type Actor%20Object%20Reference) (OtherComp :type Primitive%20Component%20Object%20Reference) (OtherBodyIndex :type Integer) (bFromSweep :type Boolean) (SweepResult :type Hit%20Result%20Structure%20%28by%20ref%29))
  (if (== (Game|Player|GetPlayerPawn 0) OtherActor)
    (Rendering|Material|SetMaterial (Variables|Default|GetStaticMesh) 0 "/Game/Images/Maps/M_Tavern.M_Tavern")))

(fn ConstructionScript)