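; BP_GM is a dialogue participant actor that runs a scripted test of the IncitingIncident dialogue on BeginPlay.
; It finds a BP_GM in the level as sole participant, prints node text and options, and chooses options by hard-coded index to advance.
; The participant interface functions are mostly stubs returning defaults, apart from the name taken from ParticipantName and a fixed Masculine gender.
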(event EventBeginPlay
  (bind _returnvalue (Actor|GetActorOfClass "BP_GM_C"))
  (bind _returnvalue_2 (Class|DlgManager|StartDialogue "/Game/Dialogue/IncitingIncident.IncitingIncident" (Utilities|Array|MakeArray _returnvalue)))
  (Development|PrintString (Utilities|String|ToString(Text) (Class|DlgContext|GetActiveNodeText _returnvalue_2)))
  (Development|PrintString (Utilities|String|ToString(Integer) (Class|DlgContext|GetOptionsNum _returnvalue_2)))
  (bind _result (Math|Integer|DecrementInt (Class|DlgContext|GetOptionsNum _returnvalue_2))
    (:%20%20
      (for _index (range 0 _result)
        (Development|PrintString (Utilities|String|ToString(Text) (Class|DlgContext|GetOptionText _returnvalue_2 _index))))
      (Class|DlgContext|ChooseOption _returnvalue_2 1)
      (Development|PrintString (Utilities|String|ToString(Text) (Class|DlgContext|GetActiveNodeText _returnvalue_2)))
      (Development|PrintString (Utilities|String|ToString(Text) (Class|DlgContext|GetOptionText _returnvalue_2)))
      (Class|DlgContext|ChooseOption _returnvalue_2))))

(fn ConstructionScript)

(fn OnDialogueEvent
  (params (Context :type Dlg%20Context%20Object%20Reference) (EventName :type Name :default "None"))
  (return false))

(fn ModifyNameValue
  (params (ValueName :type Name :default "None") (NameValue :type Name :default "None"))
  (return false))

(fn ModifyIntValue
  (params (ValueName :type Name :default "None") (bDelta :type Boolean) (Value :type Integer))
  (return false))

(fn ModifyFloatValue
  (params (ValueName :type Name :default "None") (bDelta :type Boolean) (Value :type Float%20%28single-precision%29))
  (return false))

(fn ModifyBoolValue
  (params (ValueName :type Name :default "None") (bNewValue :type Boolean))
  (return false))

(fn GetParticipantName
  (return (Utilities|String|StringToName (Variables|Default|GetParticipantName))))

(fn GetParticipantIcon
  (params (ActiveSpeaker :type Name :default "None") (ActiveSpeakerState :type Name :default "None"))
  (return 0))

(fn GetParticipantGender
  (return "Masculine"))

(fn GetParticipantDisplayName
  (params (ActiveSpeaker :type Name :default "None"))
  (return ""))

(fn GetNameValue
  (params (ValueName :type Name :default "None"))
  (return ""))

(fn GetIntValue
  (params (ValueName :type Name :default "None"))
  (return 0))

(fn GetFloatValue
  (params (ValueName :type Name :default "None"))
  (return 0.0))

(fn GetBoolValue
  (params (ValueName :type Name :default "None"))
  (return false))

(fn CheckCondition
  (params (Context :type Dlg%20Context%20Object%20Reference) (ConditionName :type Name :default "None"))
  (return false))